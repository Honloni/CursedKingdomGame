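; Footstep audio Blueprint that sets surface-specific triggers on a MetaSound footsteps manager for the player pawn.
; A looping timer starts once when the pawn moves horizontally without vertical velocity; stopping clears it, and sprinting re-sets it.
; Each step traces downward and maps the physical material's surface type to a trigger.
; Only Dirt, Concrete and the default surface continue to PlaySound2D; other surfaces just set their trigger.
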(event Custom|FootstepLoopStartEvent
  (bind _returnvalue (Game|Player|GetPlayerPawn 0))
  (bind _returnvalue_2 (Transformation|GetVelocity _returnvalue))
  (if (and (Math|Boolean|ORBoolean (> (.x _returnvalue_2) 2.0) (< (.x _returnvalue_2) -2.0) (> (.y _returnvalue_2) 2.0) (< (.y _returnvalue_2) -2.0)) (== (.z _returnvalue_2) 0.0))
    (Utilities|FlowControl|DoOnce false
      (:Completed
        (bind _returnvalue_3 (Utilities|Time|SetTimerbyEvent (delegate Custom|FootstepEvent) (Variables|Default|GetFootstepIntervall) true))
        (Variables|Default|SetFootstepTimeHandle _returnvalue_3)))))

(event Custom|FootstepLoopStopEvent
  (Utilities|Time|ClearandInvalidateTimerbyHandle (Variables|Default|GetFootstepTimeHandle))
  (Utilities|FlowControl|DoOnce false) ; enters at Reset
)

(event Custom|SprintEvent
  (bind _returnvalue (Utilities|Time|SetTimerbyEvent (delegate Custom|FootstepEvent) (Variables|Default|GetFootstepIntervall) true))
  (Variables|Default|SetFootstepTimeHandle _returnvalue))

(event Custom|FootstepEvent
  (bind _returnvalue (Game|Player|GetPlayerPawn 0))
  (bind _ms_footsteps_manager (Variables|Default|GetMS_Footsteps_Manager))
  (bind _returnvalue_2 (Transformation|GetActorLocation _returnvalue))
  (bind _outhit (Collision|LineTraceByChannel _returnvalue_2 (- _returnvalue_2 "0.000000,0.000000,200.000000") "TraceTypeQuery1" false 0 "Persistent" false))
  (Utilities|IsValid (.HitActor (Collision|BreakHitResult _outhit))
    (:Is%20Valid
      (switch Utilities|FlowControl|Switch|SwitchonEPhysicalSurface (Variables|/Script/PhysicsCore.PhysicalMaterial|GetSurfaceType (.PhysMat (Collision|BreakHitResult _outhit)))
        (:SurfaceType_Default
          (Class|AudioParameterControllerInterface|SetTriggerParameter _ms_footsteps_manager "ConcreteTrigger" :!label _label)
          (Audio|PlaySound2D (Variables|/Script/Engine.AudioComponent|GetSound _ms_footsteps_manager) 1.0 1.0 0.0 0 0 false :!label _label_2))
        (:SurfaceType1
          (goto _label))
        (:SurfaceType2
          (Class|AudioParameterControllerInterface|SetTriggerParameter _ms_footsteps_manager "DirtTrigger")
          (goto _label_2))
        (:SurfaceType3
          (Class|AudioParameterControllerInterface|SetTriggerParameter _ms_footsteps_manager "GrassTrigger"))
        (:SurfaceType4
          (Class|AudioParameterControllerInterface|SetTriggerParameter _ms_footsteps_manager "GravelTrigger"))
        (:SurfaceType5
          (Class|AudioParameterControllerInterface|SetTriggerParameter _ms_footsteps_manager "MetalTrigger"))
        (:SurfaceType6
          (Class|AudioParameterControllerInterface|SetTriggerParameter _ms_footsteps_manager "SandTrigger"))
        (:SurfaceType7
          (Class|AudioParameterControllerInterface|SetTriggerParameter _ms_footsteps_manager "TileTrigger"))
        (:SurfaceType8
          (Class|AudioParameterControllerInterface|SetTriggerParameter _ms_footsteps_manager "WaterTrigger"))
        (:SurfaceType9
          (Class|AudioParameterControllerInterface|SetTriggerParameter _ms_footsteps_manager "WoodTrigger"))))))

(fn ConstructionScript)